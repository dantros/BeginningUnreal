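; BP_PickUpSpawner is a spawner actor that scatters pickup actors at random positions when play begins.
; BeginPlay passes NumberOfActorsToSpawn to SpawnPickUps, which loops on a Counter to spawn that many instances of ActorToSpawn.
; Each spawn gets random X and Y within plus or minus SpawningArea, with no offset from the spawner's own location.
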(event `self.ReceiveBeginPlay`
  (`self.SpawnPickUps` (`self.NumberOfActorsToSpawn`)))

(fn `SpawnPickUps`
  (params (NumberOfPickUps :type Integer))
  (locals (Counter :type Integer))
  (bind _spawningarea (`self.SpawningArea`))
  (bind _returnvalue (* _spawningarea -1.0))
  (while (< (`local.Counter`) NumberOfPickUps)
    (`|SpawnActorFromClass` (`self.ActorToSpawn`) (`KismetMathLibrary.MakeTransform` (`KismetMathLibrary.MakeVector` (`KismetMathLibrary.RandomFloatInRange` _returnvalue _spawningarea) (`KismetMathLibrary.RandomFloatInRange` _returnvalue _spawningarea))) "Undefined" "MultiplyWithRoot" null null)
    (`/Engine/EditorBlueprintResources/StandardMacros.IncrementInt` (`local.Counter`))))

(fn `UserConstructionScript`)