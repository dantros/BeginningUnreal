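; Pawn Blueprint that moves along one of four world-axis directions and turns to face its direction of travel.
; Each Tick, while MovementDirection is not None, it offsets its location by the direction vector scaled by Speed and delta time, without sweeping, then snaps to the matching yaw.
; GetDirection and GetRotation map the direction enum to vectors and rotations.
; Nothing in this file sets MovementDirection.
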(event `self.ReceiveTick`
  (params (DeltaSeconds :type "Float (single-precision)"))
  (if (`|EnumInequality` (`self.MovementDirection`) "NewEnumerator0")
    ; Translation
    (bind _vectordirection (`self.GetDirection` (`self.MovementDirection`)))
    (`self.K2_SetActorLocation` (+ (* _vectordirection (* DeltaSeconds (`self.Speed`))) (`self.K2_GetActorLocation`)))
    ; Rotation
    (bind _rotator (`self.GetRotation` (`self.MovementDirection`)))
    (`self.K2_SetActorRotation` _rotator)))

(fn `GetDirection`
  (params (MovementDirection :type "/Game/Scripts/E_MovementDirection Enum" :default "NewEnumerator0"))
  (returns (VectorDirection :type "Vector Structure"))
  (switch `/Game/Scripts/E_MovementDirection` MovementDirection
    (:`NewEnumerator0`
      (return (0.0 0.0 0.0)))
    (:`NewEnumerator1`
      (return (0.0 -1.0 0.0)))
    (:`NewEnumerator2`
      (return (0.0 1.0 0.0)))
    (:`NewEnumerator3`
      (return (1.0 0.0 0.0)))
    (:`NewEnumerator4`
      (return (-1.0 0.0 0.0)))))

(fn `GetRotation`
  (params (MovementDirection :type "/Game/Scripts/E_MovementDirection Enum" :default "NewEnumerator0"))
  (returns (Rotator :type "Rotator Structure"))
  (switch `/Game/Scripts/E_MovementDirection` MovementDirection
    (:`NewEnumerator0`
      (return))
    (:`NewEnumerator1`
      (return (struct :`Yaw` -90.0)))
    (:`NewEnumerator2`
      (return (struct :`Yaw` 90.0)))
    (:`NewEnumerator3`
      (return))
    (:`NewEnumerator4`
      (return (struct :`Yaw` 180.0)))))

(fn `UserConstructionScript`)