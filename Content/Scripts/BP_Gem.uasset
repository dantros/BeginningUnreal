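; BP_Gem is a collectible gem actor that spins and disappears with a coin pickup sound when the player comes close.
; Each Tick advances its yaw by AngularSpeed scaled by delta time, then compares its distance to player pawn 0 against InteractionDistance.
; Pickup relies on this polled distance check rather than overlap events, and only destroys the gem and plays the 2D sound, with no score or inventory update.
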(event `self.ReceiveTick`
  (params (DeltaSeconds :type "Float (single-precision)"))
  (bind (_returnvalue_roll _returnvalue_pitch _returnvalue_yaw) (`KismetMathLibrary.BreakRotator` (`self.K2_GetActorRotation`)))
  ; Rotation Animation
  (`self.K2_SetActorRotation` (`KismetMathLibrary.MakeRotator` 0.0 0.0 (+ (* DeltaSeconds (`self.AngularSpeed`)) _returnvalue_yaw)))
  (if (< (`KismetMathLibrary.Vector_Distance` (`self.K2_GetActorLocation` (`GameplayStatics.GetPlayerPawn` 0)) (`self.K2_GetActorLocation`)) (`self.InteractionDistance`))
    (`self.K2_DestroyActor`)
    (`GameplayStatics.PlaySound2D` "/Game/Assets/Retro_PickUp_Coin_07.Retro_PickUp_Coin_07" 1.0 1.0 0.0 null null)))

(fn `UserConstructionScript`)