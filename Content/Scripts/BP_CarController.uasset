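; Player controller that turns Enhanced Input into a movement direction on the player's BP_Pawn.
; BeginPlay adds the IMC_CarMovement mapping context, and separate pressed and released actions exist for left, right, forward and backward.
; Presses overwrite the pawn's MovementDirection enum through MovePawn.
; Releases call StopPawn, which resets it only if that direction is still active, so the latest press wins.
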(event `self.ReceiveBeginPlay`
  (`EnhancedInputSubsystemInterface.AddMappingContext` (pcsubsystem `EnhancedInputLocalPlayerSubsystem` self) "/Game/Inputs/IMC_CarMovement.IMC_CarMovement" 0 (struct)))

(event `EnhancedInput|/Game/Inputs/IA_LeftPressed`
  (params (ActionValue :type Boolean) (ElapsedSeconds :type "Float (double-precision)") (TriggeredSeconds :type "Float (double-precision)") (InputAction :type "InputAction Object Reference" :default "/Game/Inputs/IA_LeftPressed.IA_LeftPressed"))
  (:`Triggered`
    (`self.MovePawn` "NewEnumerator1")))

(event `MovePawn`
  (params (MovementDirection :type "/Game/Scripts/E_MovementDirection Enum" :default "NewEnumerator0"))
  (bind _asbp_pawn (cast `/Game/Scripts/BP_Pawn` (`GameplayStatics.GetPlayerPawn` 0)))
  (set `/Game/Scripts/BP_Pawn.MovementDirection` MovementDirection _asbp_pawn))

(event `EnhancedInput|/Game/Inputs/IA_RightPressed`
  (params (ActionValue :type Boolean) (ElapsedSeconds :type "Float (double-precision)") (TriggeredSeconds :type "Float (double-precision)") (InputAction :type "InputAction Object Reference" :default "/Game/Inputs/IA_RightPressed.IA_RightPressed"))
  (:`Triggered`
    (`self.MovePawn` "NewEnumerator2")))

(event `EnhancedInput|/Game/Inputs/IA_ForwardPressed`
  (params (ActionValue :type Boolean) (ElapsedSeconds :type "Float (double-precision)") (TriggeredSeconds :type "Float (double-precision)") (InputAction :type "InputAction Object Reference" :default "/Game/Inputs/IA_ForwardPressed.IA_ForwardPressed"))
  (:`Triggered`
    (`self.MovePawn` "NewEnumerator3")))

(event `EnhancedInput|/Game/Inputs/IA_BackwardPressed`
  (params (ActionValue :type Boolean) (ElapsedSeconds :type "Float (double-precision)") (TriggeredSeconds :type "Float (double-precision)") (InputAction :type "InputAction Object Reference" :default "/Game/Inputs/IA_BackwardPressed.IA_BackwardPressed"))
  (:`Triggered`
    (`self.MovePawn` "NewEnumerator4")))

(event `StopPawn`
  (params (StopMovementDirection :type "/Game/Scripts/E_MovementDirection Enum" :default "NewEnumerator0"))
  (bind _asbp_pawn (cast `/Game/Scripts/BP_Pawn` (`GameplayStatics.GetPlayerPawn` 0)))
  (if (`|EnumEquality` (`/Game/Scripts/BP_Pawn.MovementDirection` _asbp_pawn) StopMovementDirection)
    (set `/Game/Scripts/BP_Pawn.MovementDirection` "NewEnumerator0" _asbp_pawn)))

(event `EnhancedInput|/Game/Inputs/IA_LeftReleased`
  (params (ActionValue :type Boolean) (ElapsedSeconds :type "Float (double-precision)") (TriggeredSeconds :type "Float (double-precision)") (InputAction :type "InputAction Object Reference" :default "/Game/Inputs/IA_LeftReleased.IA_LeftReleased"))
  (:`Triggered`
    (`self.StopPawn` "NewEnumerator1")))

(event `EnhancedInput|/Game/Inputs/IA_RightReleased`
  (params (ActionValue :type Boolean) (ElapsedSeconds :type "Float (double-precision)") (TriggeredSeconds :type "Float (double-precision)") (InputAction :type "InputAction Object Reference" :default "/Game/Inputs/IA_RightReleased.IA_RightReleased"))
  (:`Triggered`
    (`self.StopPawn` "NewEnumerator2")))

(event `EnhancedInput|/Game/Inputs/IA_ForwardReleased`
  (params (ActionValue :type Boolean) (ElapsedSeconds :type "Float (double-precision)") (TriggeredSeconds :type "Float (double-precision)") (InputAction :type "InputAction Object Reference" :default "/Game/Inputs/IA_ForwardReleased.IA_ForwardReleased"))
  (:`Triggered`
    (`self.StopPawn` "NewEnumerator3")))

(event `EnhancedInput|/Game/Inputs/IA_BackwardReleased`
  (params (ActionValue :type Boolean) (ElapsedSeconds :type "Float (double-precision)") (TriggeredSeconds :type "Float (double-precision)") (InputAction :type "InputAction Object Reference" :default "/Game/Inputs/IA_BackwardReleased.IA_BackwardReleased"))
  (:`Triggered`
    (`self.StopPawn` "NewEnumerator4")))

(fn `UserConstructionScript`)