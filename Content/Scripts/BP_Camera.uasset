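; BP_Camera is a follow camera actor that tracks the first player's pawn at a fixed world-space offset.
; On BeginPlay it stores the offset between its own location and the pawn's.
; Each Tick it sets its location to the pawn's position plus that offset, without sweep, smoothing or any change to rotation.
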(event `self.ReceiveBeginPlay`
  (set `self.Offset` (- (`self.K2_GetActorLocation`) (`self.K2_GetActorLocation` (`GameplayStatics.GetPlayerPawn` 0)))))

(event `self.ReceiveTick`
  (params (DeltaSeconds :type "Float (single-precision)"))
  (`self.K2_SetActorLocation` (+ (`self.K2_GetActorLocation` (`GameplayStatics.GetPlayerPawn` 0)) (`self.Offset`))))

(fn `UserConstructionScript`)